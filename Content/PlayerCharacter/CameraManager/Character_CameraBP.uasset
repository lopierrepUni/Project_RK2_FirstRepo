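; Player camera manager for PlayerCharacter_BP that handles first-person aim-down-sights and weapon sway.
; BlueprintUpdateCamera follows control rotation, using AimingValue to narrow FOV and blend location from the player camera to a point projected from the weapon's Ironsight socket along its forward axis.
; Tick eases a sway offset between separate idle and aiming targets, which is rotated into view space and added to the camera location.
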(event `self.ReceiveTick`
  (params (DeltaSeconds :type "Float (single-precision)"))
  (`self.CE_WeaponSway`))

(event `CE_WeaponSway`
  ;[1 1 1] Crea un pequeño offset al mover el arma
  (`/Engine/EditorBlueprintResources/StandardMacros.IsValid` (`self.Player`)
    (:`Is Valid`
      (set `self.Sway Offset` (`KismetMathLibrary.VInterpTo` (`self.Sway Offset`) (0.0 0.0 0.0) (`GameplayStatics.GetWorldDeltaSeconds`) 15.0))
      (set `self.Sway Offset` (`KismetMathLibrary.VInterpTo` (`self.Sway Offset`) (select `bool` (`/Game/PlayerCharacter/PlayerCharacter_BP.Is Aiming` (`self.Player`)) :`false` (`self.SwayIdle`) :`true` (`self.SwayADS`)) (`GameplayStatics.GetWorldDeltaSeconds`) 5.0)))))

(fn `BlueprintUpdateCamera`
  (params (CameraTarget :type "Actor Object Reference"))
  (returns (NewCameraLocation :type "Vector Structure") (NewCameraRotation :type "Rotator Structure") (NewCameraFOV :type "Float (double-precision)") (ReturnValue :type Boolean))
  (bind _returnvalue (`SceneComponent.K2_GetComponentLocation` (`/Game/PlayerCharacter/PlayerCharacter_BP.PlayerCamera` (`self.Player`))))
  (bind _location (.location (`SceneComponent.GetSocketTransform` (`/Game/Guns/WeaponBase.WeaponMesh` (`/Game/PlayerCharacter/PlayerCharacter_BP.Weapon` (`self.Player`))) "Ironsight" "RTS_World")))
  (bind _returnvalue_2 (- _location _returnvalue))
  (bind _returnvalue_3 (`KismetMathLibrary.GetForwardVector` (.rotation (`SceneComponent.GetSocketTransform` (`/Game/Guns/WeaponBase.WeaponMesh` (`/Game/PlayerCharacter/PlayerCharacter_BP.Weapon` (`self.Player`))) "Ironsight" "RTS_World"))))
  ;[1 1 1] Move the camara to aim
  (bind _asplayer_character_bp (cast `/Game/PlayerCharacter/PlayerCharacter_BP` CameraTarget))
  (bind _output_get (set `self.Player` _asplayer_character_bp))
  (`/Engine/EditorBlueprintResources/StandardMacros.IsValid` _output_get
    (:`Is Valid`
      (set `self.Final Camera Rotation` (`Pawn.GetControlRotation` (`self.Player`)))
      (set `self.Final Camera Location` (+ (`KismetMathLibrary.VLerp` _returnvalue (- _location (* _returnvalue_3 (* (`KismetMathLibrary.Dot_VectorVector` (`KismetMathLibrary.Normal` _returnvalue_2) _returnvalue_3) (/ (`KismetMathLibrary.VSize` _returnvalue_2) 250.0)))) (`/Game/PlayerCharacter/PlayerCharacter_BP.Aiming Value` (`self.Player`))) (`KismetMathLibrary.GreaterGreater_VectorRotator` (`self.Sway Offset`) (`self.Final Camera Rotation`))))
      (return (`self.Final Camera Location`) (`self.Final Camera Rotation`) (`KismetMathLibrary.Lerp` 90.0 80.0 (`/Game/PlayerCharacter/PlayerCharacter_BP.Aiming Value` (`self.Player`))) true))))

(fn `UserConstructionScript`)